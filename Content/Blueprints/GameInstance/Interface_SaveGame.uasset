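; Blueprint interface, stored with the GameInstance assets, for match state in a round-based game with two players.
; It declares getters and setters for the round count, current round, current level name and each player's win count.
; It also declares calls to restart the current level, check whether the game is finished and reset the counters.
; All functions are empty stubs, so the implementing class supplies the storage and logic.
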(fn SetRounds
  (params (Rounds :type Integer)))

(fn GetRounds
  (return 0))

(fn RestartActualLevel)

(fn SetActualLevel
  (params (LevelName :type Name)))

(fn GetActualLevel
  (return "None"))

(fn SetActualRound
  (params (Round :type Integer)))

(fn GetActualRound
  (return 0))

(fn SetPlayer0Wins
  (params (Wins :type Integer)))

(fn GetPlayer0Wins
  (return 0))

(fn SetPlayer1Wins
  (params (Wins :type Integer)))

(fn GetPlayer1Wins
  (return 0))

(fn IsGameFinished
  (return false))

(fn ResetGameCounters)