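; BP_MainFloor is a spawner that builds a breakable floor as a 3D grid of BP_BreakableFloor blocks.
; On BeginPlay, three nested loops over the horizontal, vertical and depth counts space blocks by BlocksSize from the Origin component, stacking downward in Z.
; Offsets follow world axes, while each block takes the actor's rotation and a fixed scale independent of BlocksSize.
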(event EventBeginPlay
  (bind _origin (Variables|Default|GetOrigin))
  (bind _returnvalue (Transformation|GetWorldLocation _origin))
  (for _index (range 0 (- (Variables|Default|GetHorizontalBlocksNumber) 1))
    (for _index_2 (range 0 (- (Variables|Default|GetVerticalBlocksNumber) 1))
      (for _index_3 (range 0 (- (Variables|Default|GetDepthBlocksNumber) 1))
        (Game|SpawnActorfromClass "/Game/Blueprints/Mechanics/BreakableFloor/BP_BreakableFloor.BP_BreakableFloor_C" (Math|Transform|MakeTransform (Math|Vector|MakeVector (+ (* (+ _index 1) (Variables|Default|GetBlocksSize)) (.x _returnvalue)) (+ (.y _returnvalue) (* (+ _index_2 1) (Variables|Default|GetBlocksSize))) (- (.z _returnvalue) (* (+ _index_3 1) (Variables|Default|GetBlocksSize)))) (Transformation|GetActorRotation) "6.000000,6.000000,6.000000") "Undefined" 0 0)))))

(fn ConstructionScript)