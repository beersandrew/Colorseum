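; Breakable floor tile that breaks after a random standing time or step count, or is unbreakable, and may spawn a pickup.
; The construction script randomizes its type, re-rolling Random into another; BeginPlay sets color, counter text and limit.
; Overlaps from Interface_CanBreakFloor actors track occupants and decrement steps, while Tick drives the delayed countdown when occupied.
; At zero, the plane simulates physics, then the actor is destroyed.
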(event OnComponentBeginOverlap(Box)
  (params (OverlappedComponent :type Primitive%20Component%20Object%20Reference) (OtherActor :type Actor%20Object%20Reference) (OtherComp :type Primitive%20Component%20Object%20Reference) (OtherBodyIndex :type Integer) (bFromSweep :type Boolean) (SweepResult :type Hit%20Result%20Structure%20%28by%20ref%29))
  (if (Utilities|DoesObjectImplementInterface OtherActor "/Game/Blueprints/Mechanics/BreakableFloor/Interface_CanBreakFloor.Interface_CanBreakFloor_C")
    (bind _result (Math|Integer|IncrementInt (Variables|Default|GetNumberOfPeopleOn))
      (:%20%20
        (Variables|Default|SetNumberOfPeopleOn _result)
        (switch Utilities|FlowControl|Switch|SwitchonEnum_BreakableFloorType (Variables|Default|GetType)
          (:NewEnumerator1
            (|DecreaseSteps :!label _label))
          (:NewEnumerator2
            (if (Utilities|Enum|Equal(Enum) (Variables|Default|GetSubtype) "NewEnumerator1")
              (goto _label))))))))

(event OnComponentEndOverlap(Box)
  (params (OverlappedComponent :type Primitive%20Component%20Object%20Reference) (OtherActor :type Actor%20Object%20Reference) (OtherComp :type Primitive%20Component%20Object%20Reference) (OtherBodyIndex :type Integer))
  (if (Utilities|DoesObjectImplementInterface OtherActor "/Game/Blueprints/Mechanics/BreakableFloor/Interface_CanBreakFloor.Interface_CanBreakFloor_C")
    (bind _result (Math|Integer|DecrementInt (Variables|Default|GetNumberOfPeopleOn))
      (:%20%20
        (if (<= _result 0)
          (Variables|Default|SetNumberOfPeopleOn 0)
          (else
            (Variables|Default|SetNumberOfPeopleOn _result)))))))

(event Custom|Destroy%20Block
  (Physics|SetSimulatePhysics (Variables|Default|GetPlane) true)
  (Utilities|FlowControl|Delay 1.5)
  (Actor|DestroyActor))

(event EventTick
  (params (DeltaSeconds :type Float%20%28single-precision%29))
  (if (>= (Variables|Default|GetNumberOfPeopleOn) 1)
    (switch Utilities|FlowControl|Switch|SwitchonEnum_BreakableFloorType (Variables|Default|GetType)
      (:NewEnumerator0
        (|DecreaseTime :!label _label))
      (:NewEnumerator2
        (if (Utilities|Enum|Equal(Enum) (Variables|Default|GetSubtype) "NewEnumerator0")
          (goto _label))))))

(event EventBeginPlay
  (if (>= (Math|Random|RandomIntegerinRange 0 100) (Variables|Default|GetPickupItemPct))
    _
    (else
      (Game|SpawnActorfromClass "/Game/Blueprints/Pickups/BP_PickableItem.BP_PickableItem_C" (Transformation|GetWorldTransform (Variables|Default|GetPickup)) "Undefined" 0 0)))
  (bind _returnvalue (Rendering|Material|CreateDynamicMaterialInstance (Rendering|Material|GetMaterial (Variables|Default|GetPlane) 0) "None" "None" :!class /Script/Engine.KismetMaterialLibrary))
  (Variables|Default|SetMaterial _returnvalue)
  (switch Utilities|FlowControl|Switch|SwitchonEnum_BreakableFloorType (Variables|Default|GetType)
    (:NewEnumerator0
      (Rendering|Material|SetVectorParameterValue (Variables|Default|GetMaterial) "Color" "(R=0.000000,G=0.173001,B=1.000000,A=1.000000)" :!class /Script/Engine.MaterialInstanceDynamic)
      (Rendering|Material|SetMaterial (Variables|Default|GetPlane) 0 (Variables|Default|GetMaterial))
      (Rendering|SetVisibility (Variables|Default|GetTime) true false)
      (|SetBreakTime :!label _label))
    (:NewEnumerator1
      (Rendering|Material|SetVectorParameterValue (Variables|Default|GetMaterial) "Color" "(R=1.000000,G=0.292407,B=0.000000,A=1.000000)" :!class /Script/Engine.MaterialInstanceDynamic)
      (Rendering|Material|SetMaterial (Variables|Default|GetPlane) 0 (Variables|Default|GetMaterial))
      (Rendering|SetVisibility (Variables|Default|GetSteps_txt) true false)
      (|SetSteps :!label _label_2))
    (:NewEnumerator2
      (Rendering|Material|SetVectorParameterValue (Variables|Default|GetMaterial) "Color" "(R=0.000000,G=0.210417,B=0.040536,A=1.000000)" :!class /Script/Engine.MaterialInstanceDynamic)
      (Rendering|Material|SetMaterial (Variables|Default|GetPlane) 0 (Variables|Default|GetMaterial))
      (switch int (Math|Random|RandomIntegerinRange 0 1)
        (:0
          (Variables|Default|SetSubtype "NewEnumerator0")
          (Rendering|SetVisibility (Variables|Default|Get?) true false)
          (goto _label))
        (:1
          (Variables|Default|SetSubtype "NewEnumerator0")
          (Rendering|SetVisibility (Variables|Default|Get?) true false)
          (goto _label_2))))
    (:NewEnumerator3
      (Rendering|Material|SetVectorParameterValue (Variables|Default|GetMaterial) "Color" "(R=0.531250,G=0.531250,B=0.531250,A=1.000000)" :!class /Script/Engine.MaterialInstanceDynamic)
      (Rendering|Material|SetMaterial (Variables|Default|GetPlane) 0 (Variables|Default|GetMaterial))
      (Components|DestroyComponent (Variables|Default|GetBox)))))

(fn ConstructionScript
  (bind _output_get (Variables|Default|SetType (Utilities|Select :Index (Math|Random|RandomIntegerinRange 0 3) :Option%200 "NewEnumerator0" :Option%201 "NewEnumerator1" :Option%202 "NewEnumerator2" :Option%203 "NewEnumerator3")))
  (switch Utilities|FlowControl|Switch|SwitchonEnum_BreakableFloorType _output_get
    (:NewEnumerator2
      (switch int (Math|Random|RandomIntegerinRange 0 2)
        (:0
          (Variables|Default|SetType "NewEnumerator0"))
        (:1
          (Variables|Default|SetType "NewEnumerator1"))
        (:2
          (Variables|Default|SetType "NewEnumerator3"))))))

(fn UpdateDisplayTime
  (params (Time :type Float%20%28double-precision%29))
  (Rendering|Components|TextRender|SetText (Variables|Default|GetTime) (Utilities|Text|ToText(Float) Time "HalfToEven" false true 1 1 0 1)))

(fn UpdateDisplaySteps
  (params (Steps :type Integer))
  (Rendering|Components|TextRender|SetText (Variables|Default|GetSteps_txt) (Utilities|Text|ToText(Integer) Steps)))