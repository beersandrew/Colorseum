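; Armor pickup actor that grants an armor increment to any overlapping actor implementing the PlayersHealth_BPI interface.
; On overlap it reads the actor's armor through the interface, increments it and writes it back.
; It then notifies its SpawnedBy reference with PickItemMessage and destroys itself.
; The collection sound and particle nodes, along with a debug print, are present but unconnected.
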(event Collision|EventActorBeginOverlap
  (params (OtherActor :type Actor%20Object%20Reference))
  (if (Utilities|DoesObjectImplementInterface OtherActor "/Game/Blueprints/UI/BlueprintInterfaces/PlayersHealth_BPI.PlayersHealth_BPI_C")
    (bind _armor (Class|PlayersHealthBPI|GetArmor(Message) OtherActor))
    (bind _result (Math|Integer|IncrementInt _armor)
      (:%20%20
        (Class|PlayersHealthBPI|SetArmor(Message) OtherActor _result)
        (Class|InterfacePickupSpot|PickItem(Message) (Variables|Default|GetSpawnedBy))
        (Actor|DestroyActor)))))

(fn ConstructionScript)

(fn GetPlayerIndex
  (return 0))