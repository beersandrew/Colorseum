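; Health pickup Blueprint that restores one point of health to an overlapping actor implementing PlayersHealth_BPI.
; On overlap it reads current and max health through the interface, and only when below max sets the incremented value.
; It then notifies its SpawnedBy reference through PickItemMessage and destroys itself.
; The sound, particle and debug print nodes are present but unconnected, so they never run.
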(event Collision|EventActorBeginOverlap
  (params (OtherActor :type Actor%20Object%20Reference))
  (if (Utilities|DoesObjectImplementInterface OtherActor "/Game/Blueprints/UI/BlueprintInterfaces/PlayersHealth_BPI.PlayersHealth_BPI_C")
    (bind _maxhealth (Class|PlayersHealthBPI|GetMaxHealth(Message) OtherActor))
    (bind _health (Class|PlayersHealthBPI|GetHealth(Message) OtherActor))
    (if (< _health _maxhealth)
      (bind _health_2 (Class|PlayersHealthBPI|GetHealth(Message) OtherActor))
      (bind _result (Math|Float|IncrementFloat _health_2)
        (:%20%20
          (Class|PlayersHealthBPI|SetHealth(Message) OtherActor _result)
          (Class|InterfacePickupSpot|PickItem(Message) (Variables|Default|GetSpawnedBy))
          (Actor|DestroyActor))))))

(fn ConstructionScript)