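; BP_PickableItem is a placeable spawner that puts a random pickup into the level when play begins.
; On BeginPlay it rolls an integer from 1 to ItemsTypeCount and spawns a speed, armor or health pickup at its root component's world transform.
; The pickup classes are hardcoded in the switch, and the spawner stays in the level after spawning.
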(event EventBeginPlay
  (switch int (Math|Random|RandomIntegerinRange 1 (Variables|Default|GetItemsTypeCount))
    (:1
      (Game|SpawnActorfromClass "/Game/Blueprints/Pickups/SpeedPickup_BP.SpeedPickup_BP_C" (Transformation|GetWorldTransform (Variables|Default|GetDefaultSceneRoot)) "Undefined" 0 0))
    (:2
      (Game|SpawnActorfromClass "/Game/Blueprints/Pickups/BP_ArmorPickup.BP_ArmorPickup_C" (Transformation|GetWorldTransform (Variables|Default|GetDefaultSceneRoot)) "Undefined" 0 0))
    (:3
      (Game|SpawnActorfromClass "/Game/Blueprints/Pickups/BP_HealthPickup.BP_HealthPickup_C" (Transformation|GetWorldTransform (Variables|Default|GetDefaultSceneRoot)) "Undefined" 0 0))))

(fn ConstructionScript)