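; SpeedPickup_BP is a speed boost pickup whose mesh bobs up and down continuously through looping MoveComponentTo calls.
; On overlap with an actor implementing PlayerSpeed_BPI, it sends that actor the speed message, notifies SpawnedBy that the item was picked, then destroys itself.
; The collection sound and emitter nodes are present but disconnected, so they never play.
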(event Collision|EventActorBeginOverlap
  (params (OtherActor :type Actor%20Object%20Reference))
  (if (Utilities|DoesObjectImplementInterface OtherActor "/Game/Blueprints/UI/BlueprintInterfaces/PlayerSpeed_BPI.PlayerSpeed_BPI_C")
    (Class|PlayerSpeedBPI|Player'sSpeed(Message) OtherActor)
    (Class|InterfacePickupSpot|PickItem(Message) (Variables|Default|GetSpawnedBy))
    (Actor|DestroyActor)))

(event EventBeginPlay
  (Components|MoveComponentTo (Variables|Default|GetSpeedPickup_SM) (Variables|Default|GetGoing%20Up) "0, 0, 0" false false (Variables|Default|GetMove%20Speed) false :!label _label)
  (Components|MoveComponentTo (Variables|Default|GetSpeedPickup_SM) (Variables|Default|GetGoing%20Down) "0, 0, 0" false false (Variables|Default|GetMove%20Speed) false)
  (goto _label))

(fn ConstructionScript)