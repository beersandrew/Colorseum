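; Pickup spot that spawns a health, armor or speed pickup at ItemLocation on BeginPlay, either fixed by ItemType or picked at random.
; Each pickup receives a SpawnedBy reference to the spot, and PickItem marks the spot empty.
; While empty with ReSpawn enabled, Tick uses a Delay to count down in TickDelay steps, printing the remaining time, then spawns again and resets the timer.
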(event EventBeginPlay
  (CallFunction|SpawnItem))

(event EventTick
  (params (DeltaSeconds :type Float%20%28single-precision%29))
  (if (Variables|Default|GetReSpawn)
    (if (not (Variables|Default|GetItemInside))
      (Utilities|FlowControl|Delay (Variables|Default|GetTickDelay))
      (if (<= (- (Variables|Default|GetSecondsRemainingsToSpawn) (Variables|Default|GetTickDelay)) 0.0)
        (CallFunction|SpawnItem)
        (else
          (bind _output_get (Variables|Default|SetSecondsRemainingsToSpawn (- (Variables|Default|GetSecondsRemainingsToSpawn) (Variables|Default|GetTickDelay))))
          (Development|PrintString (Utilities|String|ToString(Float) _output_get)))))))

(event EventPickItem
  (Variables|Default|SetItemInside false))

(fn ConstructionScript)

(fn SpawnItem
  (Variables|Default|SetSecondsRemainingsToSpawn (Variables|Default|GetSpawnAfterSeconds))
  (Variables|Default|SetItemInside true)
  (switch Utilities|FlowControl|Switch|SwitchonEnum_ItemPickableType (Variables|Default|GetItemType)
    (:NewEnumerator0
      (switch int (Math|Random|RandomIntegerinRange 0 2)
        (:0
          (bind _returnvalue (Game|SpawnActorfromClass "/Game/Blueprints/Pickups/BP_HealthPickup.BP_HealthPickup_C" (Transformation|GetWorldTransform (Variables|Default|GetItemLocation)) "Undefined" 0 0 :!label _label))
          (Variables|/Game/Blueprints/Pickups/BP_HealthPickup.BP_HealthPickup_C|SetSpawnedBy _returnvalue self))
        (:1
          (bind _returnvalue_2 (Game|SpawnActorfromClass "/Game/Blueprints/Pickups/BP_ArmorPickup.BP_ArmorPickup_C" (Transformation|GetWorldTransform (Variables|Default|GetItemLocation)) "Undefined" 0 0 :!label _label_2))
          (Variables|/Game/Blueprints/Pickups/BP_ArmorPickup.BP_ArmorPickup_C|SetSpawnedBy _returnvalue_2 self))
        (:2
          (bind _returnvalue_3 (Game|SpawnActorfromClass "/Game/Blueprints/Pickups/SpeedPickup_BP.SpeedPickup_BP_C" (Transformation|GetWorldTransform (Variables|Default|GetItemLocation)) "Undefined" 0 0 :!label _label_3))
          (Variables|/Game/Blueprints/Pickups/SpeedPickup_BP.SpeedPickup_BP_C|SetSpawnedBy _returnvalue_3 self))))
    (:NewEnumerator1
      (goto _label))
    (:NewEnumerator2
      (goto _label_2))
    (:NewEnumerator3
      (goto _label_3))))