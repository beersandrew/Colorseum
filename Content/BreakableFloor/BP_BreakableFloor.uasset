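; Breakable floor tile that destroys itself after a randomized amount of standing time or number of steps.
; A box trigger counts overlapping actors implementing an interface; Tick drives the delayed countdown, while begin overlap decrements steps, both updating text displays.
; Type sets the dynamic material's color and break rule, including a random-subtype variant and an inert one without a trigger.
; BeginPlay also rolls a percentage chance to spawn a BP_PickableItem.
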(event OnComponentBeginOverlap(Box)
  (params (OverlappedComponent :type Primitive%20Component%20Object%20Reference) (OtherActor :type Actor%20Object%20Reference) (OtherComp :type Primitive%20Component%20Object%20Reference) (OtherBodyIndex :type Integer) (bFromSweep :type Boolean) (SweepResult :type Hit%20Result%20Structure%20%28by%20ref%29))
  (if (Utilities|DoesObjectImplementInterface OtherActor 0)
    (bind _result (Math|Integer|IncrementInt (Variables|Default|GetNumberOfPeopleOn))
      (:%20%20
        (Variables|Default|SetNumberOfPeopleOn _result)
        (switch Utilities|FlowControl|Switch|Switchon (Variables|Default|GetType)
          (:NewEnumerator1
            (|DecreaseSteps :!label _label))
          (:NewEnumerator2
            (if (Utilities|Enum|Equal(Enum) 0 0)
              (goto _label))))))))

(event OnComponentEndOverlap(Box)
  (params (OverlappedComponent :type Primitive%20Component%20Object%20Reference) (OtherActor :type Actor%20Object%20Reference) (OtherComp :type Primitive%20Component%20Object%20Reference) (OtherBodyIndex :type Integer))
  (if (Utilities|DoesObjectImplementInterface OtherActor 0)
    (bind _result (Math|Integer|DecrementInt (Variables|Default|GetNumberOfPeopleOn))
      (:%20%20
        (if (<= _result 0)
          (Variables|Default|SetNumberOfPeopleOn 0)
          (else
            (Variables|Default|SetNumberOfPeopleOn _result)))))))

(event Custom|Destroy%20Block
  (Actor|DestroyActor))

(event EventTick
  (params (DeltaSeconds :type Float%20%28single-precision%29))
  (if (>= (Variables|Default|GetNumberOfPeopleOn) 1)
    (switch Utilities|FlowControl|Switch|Switchon (Variables|Default|GetType)
      (:NewEnumerator0
        (|DecreaseTime :!label _label))
      (:NewEnumerator2
        (if (Utilities|Enum|Equal(Enum) 0 0)
          (goto _label))))))

(event EventBeginPlay
  (bind _returnvalue (Rendering|Material|CreateDynamicMaterialInstance (Rendering|Material|GetMaterial (Variables|Default|GetPlane) 0) "None" "None" :!class /Script/Engine.KismetMaterialLibrary))
  (Variables|Default|SetMaterial _returnvalue)
  (|SetPickup)
  (|SetFloorType))

(fn ConstructionScript
  (switch Utilities|FlowControl|Switch|Switchon (Variables|Default|GetType)
    (:NewEnumerator2
      (switch int (Math|Random|RandomIntegerinRange 0 3)
        (:0
          (Variables|Default|SetType 0))
        (:1
          (Variables|Default|SetType 0))
        (:2
          (Variables|Default|SetType 0))
        (:3
          (Variables|Default|SetType 0))))))

(fn UpdateDisplayTime
  (params (Time :type Float%20%28double-precision%29))
  (Rendering|Components|TextRender|SetText (Variables|Default|GetTime) (Utilities|Text|ToText(Float) Time "HalfToEven" false true 1 1 0 1)))

(fn UpdateDisplaySteps
  (params (Steps :type Integer))
  (Rendering|Components|TextRender|SetText (Variables|Default|GetSteps_txt) (Utilities|Text|ToText(Integer) Steps)))